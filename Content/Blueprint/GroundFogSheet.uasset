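; GroundFogSheet is a placeable ground fog card whose look is set per instance through its variables.
; The construction script assigns the fog mesh, applies world scale, and creates a dynamic instance of CI_GroundFogCard.
; It pushes color, smoke texture, depth and distance fading, radial mask, fresnel, UV distortion, tiling and noise speed into that material.
; The event graph holds only disabled stubs, so the Blueprint runs no gameplay logic.
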(event EventBeginPlay)

(event Collision|EventActorBeginOverlap
  (params (OtherActor :type Actor%20Object%20Reference)))

(event EventTick
  (params (DeltaSeconds :type Float%20%28single-precision%29)))

(fn ConstructionScript
  (bind _staticmesh (Variables|Default|GetStaticMesh))
  (Components|StaticMesh|SetStaticMesh _staticmesh (Variables|Setup|GetFogMesh))
  (bind _returnvalue (Rendering|Material|CreateDynamicMaterialInstance _staticmesh 0 "/Game/Completed/Materials/Instances/CI_GroundFogCard.CI_GroundFogCard" "None" :!class /Script/Engine.PrimitiveComponent))
  (Variables|Setup|SetGroundFogMID _returnvalue)
  (Transformation|SetWorldScale3D _staticmesh (Variables|Setup|GetScale))
  (Rendering|Material|SetVectorParameterValue (Variables|Setup|GetGroundFogMID) "Color" (Variables|Material|GetFogColour) :!class /Script/Engine.MaterialInstanceDynamic)
  (Rendering|Material|SetTextureParameterValue (Variables|Setup|GetGroundFogMID) "SmokeTexture" (Variables|Material|GetFogTexture))
  (Rendering|Material|SetScalarParameterValue (Variables|Setup|GetGroundFogMID) "DepthFadeDistance" (Variables|Material|GetDepthFadeDistance) :!class /Script/Engine.MaterialInstanceDynamic)
  (Rendering|Material|SetScalarParameterValue (Variables|Setup|GetGroundFogMID) "FadeDistanceOffset" (Variables|Material|GetFadeDistanceOffset) :!class /Script/Engine.MaterialInstanceDynamic)
  (Rendering|Material|SetScalarParameterValue (Variables|Setup|GetGroundFogMID) "FadingDistance" (Variables|Material|GetFadingDistance) :!class /Script/Engine.MaterialInstanceDynamic)
  (Rendering|Material|SetScalarParameterValue (Variables|Setup|GetGroundFogMID) "FogRadialGradientStrength" (Variables|Material|GetFogRadialMaskStrength) :!class /Script/Engine.MaterialInstanceDynamic)
  (Rendering|Material|SetScalarParameterValue (Variables|Setup|GetGroundFogMID) "FogUVDistortion" (Variables|Material|GetFogUVDistortion) :!class /Script/Engine.MaterialInstanceDynamic)
  (Rendering|Material|SetScalarParameterValue (Variables|Setup|GetGroundFogMID) "FogFresnelAngle" (Variables|Material|GetFogFresnelAngle) :!class /Script/Engine.MaterialInstanceDynamic)
  (Rendering|Material|SetScalarParameterValue (Variables|Setup|GetGroundFogMID) "FogTiling" (Variables|Material|GetFogTiling) :!class /Script/Engine.MaterialInstanceDynamic)
  (Rendering|Material|SetScalarParameterValue (Variables|Setup|GetGroundFogMID) "FogNoiseTiling" (Variables|Material|GetFogNoiseTiling) :!class /Script/Engine.MaterialInstanceDynamic)
  (Rendering|Material|SetScalarParameterValue (Variables|Setup|GetGroundFogMID) "FogNoiseSpeedX" (Variables|Material|GetFogNoiseSpeedX) :!class /Script/Engine.MaterialInstanceDynamic)
  (Rendering|Material|SetScalarParameterValue (Variables|Setup|GetGroundFogMID) "FogNoiseSpeedY" (Variables|Material|GetFogNoiseSpeedY) :!class /Script/Engine.MaterialInstanceDynamic))